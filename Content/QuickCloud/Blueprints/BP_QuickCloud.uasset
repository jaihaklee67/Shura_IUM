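; BP_QuickCloud is a volumetric cloud actor that renders a Sparse Volume Texture through the M_QuicklyCloud material on QuickCloudCore.
; SetUp creates a dynamic material instance and pushes scattering, density, optional ambient-light mixing and shadow settings, remapping Beer's-powder through a logistic curve.
; It also sets global console variables for Lumen indirect lighting and visible distance.
; SetUp runs on construction and every Tick, recreating the instance each time.
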(event EventBeginPlay)

(event Collision|EventActorBeginOverlap
  (params (OtherActor :type Actor%20Object%20Reference)))

(event EventTick
  (params (DeltaSeconds :type Float%20%28single-precision%29))
  (BasicFunctions|SetUp))

(fn ConstructionScript
  (BasicFunctions|SetUp))

(fn SetUp
  (bind _cvar_lumen_indirectlighting_support (Variables|GlobalCvar|GetCvar_Lumen_IndirectLighting_Support))
  (Utilities|FlowControl|Sequence
    (:then_0
      (bind _returnvalue (Rendering|Material|CreateDynamicMaterialInstance (Variables|Default|GetQuickCloud_Core) 0 "/Game/QuickCloud/Materials/M_QuicklyCloud.M_QuicklyCloud" "None" :!class /Script/Engine.PrimitiveComponent))
      (Variables|GlobalBasicSettings|SetVDB_Clouds_Material_Instance _returnvalue))
    (:then_1
      (Class|MaterialInstanceDynamic|SetSparseVolumeTextureParameterValue (Variables|GlobalBasicSettings|GetVDB_Clouds_Material_Instance) "Input SVT" (Variables|BasicControls|GetSparse_Volume_Texture))
      (Rendering|Material|SetVectorParameterValue (Variables|GlobalBasicSettings|GetVDB_Clouds_Material_Instance) "Scattering Color" (Variables|BasicControls|GetScattering_Color) :!class /Script/Engine.MaterialInstanceDynamic)
      (Rendering|Material|SetScalarParameterValue (Variables|GlobalBasicSettings|GetVDB_Clouds_Material_Instance) "Scattering Intensity" (Variables|BasicControls|GetScattering_Intensity) :!class /Script/Engine.MaterialInstanceDynamic)
      (Rendering|Material|SetScalarParameterValue (Variables|GlobalBasicSettings|GetVDB_Clouds_Material_Instance) "Density" (Variables|BasicControls|GetDensity) :!class /Script/Engine.MaterialInstanceDynamic)
      (Rendering|Material|SetScalarParameterValue (Variables|GlobalBasicSettings|GetVDB_Clouds_Material_Instance) "Thick" (/ (Variables|BasicControls|GetExtinction) 1e+01) :!class /Script/Engine.MaterialInstanceDynamic))
    (:then_2
      (if (Variables|AmbientLightMixing|GetUse_Ambient_Light_Mixing)
        (Rendering|Material|SetScalarParameterValue (Variables|GlobalBasicSettings|GetVDB_Clouds_Material_Instance) "Sun Intensity" (/ (Variables|AmbientLightMixing|GetLight_Intensity_Multiplier) 1e+01) :!class /Script/Engine.MaterialInstanceDynamic)
        (Rendering|Material|SetScalarParameterValue (Variables|GlobalBasicSettings|GetVDB_Clouds_Material_Instance) "Sun Contribution" (Variables|AmbientLightMixing|GetLight_Color_Saturation) :!class /Script/Engine.MaterialInstanceDynamic)
        (Rendering|Material|SetVectorParameterValue (Variables|GlobalBasicSettings|GetVDB_Clouds_Material_Instance) "Sun Color" (Variables|AmbientLightMixing|GetLight_Color_Multiplier) :!class /Script/Engine.MaterialInstanceDynamic)
        (Rendering|Material|SetScalarParameterValue (Variables|GlobalBasicSettings|GetVDB_Clouds_Material_Instance) "sky Light Leaking" (Variables|AmbientLightMixing|GetSky_Light_Leaking) :!class /Script/Engine.MaterialInstanceDynamic)
        (Rendering|Material|SetVectorParameterValue (Variables|GlobalBasicSettings|GetVDB_Clouds_Material_Instance) "Sky Light Color" (Variables|AmbientLightMixing|GetSky_Light_Color_Multiplier) :!class /Script/Engine.MaterialInstanceDynamic)
        (Rendering|Material|SetScalarParameterValue (Variables|GlobalBasicSettings|GetVDB_Clouds_Material_Instance) "Sky Light Saturation" (Variables|AmbientLightMixing|GetSky_Light_Saturation) :!class /Script/Engine.MaterialInstanceDynamic)))
    (:then_3
      (bind _process (BasicFunctions|ParameterBeersPowder (Variables|BasicControls|GetBeers_Powder_Effect) 3e+01 -0.2 7e+01))
      (Rendering|Material|SetScalarParameterValue (Variables|GlobalBasicSettings|GetVDB_Clouds_Material_Instance) "Beers Powder Intensity" _process :!class /Script/Engine.MaterialInstanceDynamic)
      (Rendering|Material|SetVectorParameterValue (Variables|GlobalBasicSettings|GetVDB_Clouds_Material_Instance) "Self Shadow Color" (Variables|BasicControls|GetDetail_Shadow_Color) :!class /Script/Engine.MaterialInstanceDynamic)
      (Rendering|Material|SetScalarParameterValue (Variables|GlobalBasicSettings|GetVDB_Clouds_Material_Instance) "Self Shadow Intensity" (Variables|BasicControls|GetDetail_Shadow) :!class /Script/Engine.MaterialInstanceDynamic)
      (Rendering|SetCastShadow (Variables|Default|GetQuickCloud_Core) (Variables|BasicControls|GetCast_Shadow)))
    (:then_4
      (if (Variables|GlobalRenderingSettings|GetLumen_IndirectLighting_Support)
        (bind _return_value (BasicFunctions|CvarAppend _cvar_lumen_indirectlighting_support "1"))
        (Development|ExecuteConsoleCommand _return_value 0)
        (else
          (bind _return_value_2 (BasicFunctions|CvarAppend _cvar_lumen_indirectlighting_support "0"))
          (Development|ExecuteConsoleCommand _return_value_2 0))))
    (:then_5
      (bind _return_value_3 (BasicFunctions|CvarAppend (Variables|GlobalCvar|GetCvar_Visible_Distance) (Utilities|String|ToString(Float) (Variables|GlobalRenderingSettings|GetVisible_Distance))))
      (Development|ExecuteConsoleCommand _return_value_3 0))))

(fn CvarAppend
  (params (Cvar%20Body :type String) (Cvar%20Value :type String))
  (return (Utilities|String|Append Cvar%20Body " " Cvar%20Value)))

(fn ParameterBeersPowder
  (params (original :type Float%20%28double-precision%29) (a :type Float%20%28double-precision%29) (k :type Float%20%28double-precision%29) (x0 :type Float%20%28double-precision%29))
  (return (/ a (+ 1.0 (Class|KismetMathLibrary|Exp (* k (- (- 6e+01 original) x0)))))))